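; Player controller Blueprint that opens the inventory screen when the Inventory input action is pressed.
; It creates WBP_Inventory on first use, caches it, then adds it to the viewport, shows the mouse cursor and switches to UI-only input focused on the widget.
; It has no logic for closing the inventory or restoring game input, and a Game and UI input mode node is left unconnected.
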(event EventBeginPlay)

(event EventTick
  (params (DeltaSeconds :type Float%20%28single-precision%29)))

(event Input|ActionEvents|InputActionInventory
  (params (Key :type Key%20Structure :default "None"))
  (:Pressed
    (Utilities|IsValid (Variables|Default|GetInventoryWidget)
      (:Is%20Valid
        _)
      (:Is%20Not%20Valid
        (bind _returnvalue (UserInterface|CreateWidget "/Game/Widget/InvenWidget/WBP_Inventory.WBP_Inventory_C"))
        (Variables|Default|SetInventoryWidget _returnvalue)))
    (UserInterface|Viewport|AddtoViewport (Variables|Default|GetInventoryWidget) 0)
    (Variables|Default|SetbShowMouseCursor true)
    (Input|SetInputModeUIOnly self (Variables|Default|GetInventoryWidget) "DoNotLock")))

(fn ConstructionScript)